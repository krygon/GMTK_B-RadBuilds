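; BP_DataPad is an interactable data pad that shows readable text on screen when clicked.
; Clicking its BPC_InteractionTrigger component creates a HUD_DataPad widget and adds it to the viewport.
; The SelectText enum is converted to a row name to look up content in Datapad_DT for the widget's TextContent.
; The row name is also printed as debug output.
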(event `self.BPC_InteractionTrigger.OnClicked`
  (params (TouchedComponent :type "PrimitiveComponent Object Reference") (ButtonPressed :type "Key Structure"))
  (bind _returnvalue (`KismetStringLibrary.Conv_StringToName` (`|GetEnumeratorNameAsString` (`self.Select_Text`))))
  (bind _returnvalue_2 (`|CreateWidget` "/Game/Ricardo/UI/DataPad/HUD_DataPad.HUD_DataPad_C"))
  (bind _output_get (set `self.DataPadUI` _returnvalue_2))
  (`UserWidget.AddToViewport` _output_get 0)
  (bind _returnvalue_3 (`|GetDataTableRow` "/Game/Ricardo/UI/DataPad/Datapad_DT.Datapad_DT" _returnvalue)
    (:`then`
      _)
    (:`RowNotFound`
      _))
  (set `/Game/Ricardo/UI/DataPad/HUD_DataPad.Text_Content` (`.DataPad_Content_Text_3_5E3470A4409F2874DB966EBCB27E044E` (break `/Game/Ricardo/UI/DataPad/DataPad_Strut` _returnvalue_3)) (`self.DataPadUI`))
  (`KismetSystemLibrary.PrintString` (`KismetStringLibrary.Conv_NameToString` _returnvalue)))

(fn `UserConstructionScript`)