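; Jail door actor that blocks passage with lasers and a collider, driven by an interaction component.
; BeginPlay binds the component's start and stop action events, with OpenDoor and CloseDoor as the door handlers.
; Opening always plays a sound, but hides the lasers and disables collision only when unlocked.
; Closing plays the same sound and shows the lasers again, without re-enabling collision.
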(event `self.ReceiveBeginPlay`
  (bind _bpc_interactionactor (`self.BPC_InteractionActor`))
  (add `/Game/Dan/TopDownBP/Blueprints/Components/Interactions/BPC_InteractionActor.StartAction` _bpc_interactionactor (`|CreateDelegate` :!event `Open Door`))
  (add `/Game/Dan/TopDownBP/Blueprints/Components/Interactions/BPC_InteractionActor.StopAction` _bpc_interactionactor (`|CreateDelegate` :!event `Close Door`)))

(event `Open Door`
  (if (`self.IsLocked`)
    (`GameplayStatics.PlaySound2D` "/Game/Ricardo/Audio/SFX/ES_Sci_Fi_Spaceship_10_-_SFX_Producer.ES_Sci_Fi_Spaceship_10_-_SFX_Producer" 0.7 1.0 0.0 null null)
    (else
      (`GameplayStatics.PlaySound2D` "/Game/Ricardo/Audio/SFX/ES_Sci_Fi_Spaceship_10_-_SFX_Producer.ES_Sci_Fi_Spaceship_10_-_SFX_Producer" 0.7 1.0 0.0 null null)
      (`SceneComponent.SetHiddenInGame` (`self.Lasers`) true true)
      (`PrimitiveComponent.SetCollisionEnabled` (`self.Collider`) "NoCollision"))))

(event `Close Door`
  (`GameplayStatics.PlaySound2D` "/Game/Ricardo/Audio/SFX/ES_Sci_Fi_Spaceship_10_-_SFX_Producer.ES_Sci_Fi_Spaceship_10_-_SFX_Producer" 0.7 1.0 0.0 null null)
  (`SceneComponent.SetHiddenInGame` (`self.Lasers`) false true))

(fn `UserConstructionScript`)