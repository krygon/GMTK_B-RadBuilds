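; BP_Control_Panel_Camera is an interactable control panel that opens and closes a security camera console UI.
; Collide-interact events from its interaction trigger component show the UI, interact events pass their on/off state through, and CloseComputer hides it.
; All three route through ToggleConsoleUI, which forwards the state to the security cameras component and resets the trigger whenever the UI is shown.
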(event `self.ReceiveBeginPlay`)

(event `self.BPC_InteractionTrigger.OnCollideInteract`
  (`self.ToggleConsoleUI` true))

(event `self.BPC_InteractionTrigger.OnInteract`
  (params (On :type Boolean))
  (`self.ToggleConsoleUI` On))

(event `Close Computer`
  (`self.ToggleConsoleUI` false))

(fn `ToggleConsoleUI`
  (params (InShow :type Boolean))
  (`/Game/Dan/TopDownBP/Blueprints/Components/SecurityCameras/BPC_SecurityCameras.ToggleUI` (`self.BPC_SecurityCameras`) InShow)
  (if (`local.InShow`)
    (`/Game/Dan/TopDownBP/Blueprints/Components/Interactions/BPC_InteractionTrigger.Reset` (`self.BPC_InteractionTrigger`))))

(fn `UserConstructionScript`)