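; Sci-fi sliding door that opens when a Player-tagged component enters its trigger box and closes when it leaves, unless locked.
; A timeline lerps the door mesh's relative Z, reversing mid-motion if needed, with a 2D sound pitched lower on closing.
; The construction script creates dynamic materials on door and arch, coloured red if locked or green if unlocked.
; UnlockDoor clears the lock and turns both green.
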(event `self.ReceiveBeginPlay`
  (`TimelineComponent.SetPlayRate` (`self.OpenCloseDoor_Timeline`) (/ 1.0 0.75)))

(event `self.Box.OnComponentBeginOverlap`
  (params (OverlappedComponent :type "PrimitiveComponent Object Reference") (OtherActor :type "Actor Object Reference") (OtherComp :type "PrimitiveComponent Object Reference") (OtherBodyIndex :type Integer) (bFromSweep :type Boolean) (SweepResult :type "HitResult Structure (by ref)"))
  (if (`ActorComponent.ComponentHasTag` OtherComp "Player")
    (if (not (`self.IsLocked`))
      (`self.OpenDoor`)
      (`GameplayStatics.PlaySound2D` "/Game/Ricardo/Audio/SFX/ES_Sci_Fi_Spaceship_10_-_SFX_Producer.ES_Sci_Fi_Spaceship_10_-_SFX_Producer" 0.7 1.0 0.0 null null))))

(event `OpenDoor`
  (if (`TimelineComponent.IsPlaying` (`self.OpenCloseDoor_Timeline`))
    (bind (_direction _newtrack_0) (`Timeline|OpenCloseDoor_Timeline` :!label _label)
      (:`Update`
        (`SceneComponent.K2_SetRelativeTransform` (`self.SciFi_Door_Door`) (`KismetMathLibrary.MakeTransform` (`KismetMathLibrary.MakeVector` 0.0 0.0 (`KismetMathLibrary.Lerp` (`self.Door_Normal`) (`self.LowerDoorAMount`) _newtrack_0))) false false)))
    (else
      (goto _label :!via `PlayFromStart`))))

(event `CloseDoor`
  (if (`TimelineComponent.IsPlaying` (`self.OpenCloseDoor_Timeline`))
    (goto _label :!via `Reverse`)
    (else
      (goto _label :!via `ReverseFromEnd`))))

(event `self.Box.OnComponentEndOverlap`
  (params (OverlappedComponent :type "PrimitiveComponent Object Reference") (OtherActor :type "Actor Object Reference") (OtherComp :type "PrimitiveComponent Object Reference") (OtherBodyIndex :type Integer))
  (if (`ActorComponent.ComponentHasTag` OtherComp "Player")
    (if (not (`self.IsLocked`))
      (`self.CloseDoor`)
      (`GameplayStatics.PlaySound2D` "/Game/Ricardo/Audio/SFX/ES_Sci_Fi_Spaceship_10_-_SFX_Producer.ES_Sci_Fi_Spaceship_10_-_SFX_Producer" 0.7 0.8 0.0 null null))))

(event `UnlockDoor`
  (set `self.IsLocked` false)
  (`MaterialInstanceDynamic.SetVectorParameterValue` (`self.DoorMaterial`) "Colour" (struct :`G` 1.0 :`A` 1.0))
  (`MaterialInstanceDynamic.SetVectorParameterValue` (`self.DoorArchMaterial`) "Colour" (struct :`G` 1.0 :`A` 1.0)))

(fn `UserConstructionScript`
  (bind _doormaterial (`self.DoorMaterial`))
  (bind _doorarchmaterial (`self.DoorArchMaterial`))
  (bind _returnvalue (`PrimitiveComponent.CreateDynamicMaterialInstance` (`self.SciFi_Door_Door`) 1 null "None"))
  (set `self.DoorMaterial` _returnvalue)
  (bind _returnvalue_2 (`PrimitiveComponent.CreateDynamicMaterialInstance` (`self.SciFi_Door_DoorArch`) 1 null "None"))
  (set `self.DoorArchMaterial` _returnvalue_2)
  (if (`self.IsLocked`)
    (`MaterialInstanceDynamic.SetVectorParameterValue` _doormaterial "Colour" (struct :`R` 1.0 :`A` 1.0))
    (`MaterialInstanceDynamic.SetVectorParameterValue` _doorarchmaterial "Colour" (struct :`R` 1.0 :`A` 1.0))
    (else
      (`MaterialInstanceDynamic.SetVectorParameterValue` _doormaterial "Colour" (struct :`G` 1.0 :`A` 1.0))
      (`MaterialInstanceDynamic.SetVectorParameterValue` _doorarchmaterial "Colour" (struct :`G` 1.0 :`A` 1.0)))))