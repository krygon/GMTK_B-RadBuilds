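; Lift actor that moves a platform between Point A and Point B, starting at the end chosen by StartingLocation.
; A timeline lerps the platform's relative location, with play rate set from the travel time and direction set by playing forward or reversing.
; Cube clicks toggle direction when a pawn is in the box, while two interaction components trigger each direction, skipping the range check and IsAtA update.
; IsLocked blocks movement and its sound.
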(event `self.ReceiveTick`
  (params (DeltaSeconds :type "Float (single-precision)")))

(event `self.ReceiveBeginPlay`
  ;[1 1 1] Set Variables
  (`TimelineComponent.SetPlayRate` (`self.Lift_Timeline`) (/ 1.0 (`self.Lift_Time_To_Desitnation`)))
  (set `self.Point_A_Location` (`SceneComponent.RelativeLocation` (`self.Point - A`)))
  (set `self.Point_B_Location` (`SceneComponent.RelativeLocation` (`self.Point - B`)))
  ;[1 1 1] Set up Start Position switch Reset Lift Position
  (switch `int` (`self.Starting Location`)
    (:`0`
      (set `self.Lift_Current_Location` (`self.Point_A_Location`)))
    (:`1`
      (set `self.Lift_Current_Location` (`self.Point_B_Location`))))
  (`SceneComponent.K2_SetRelativeLocation` (`self.Lift_Platform_Main`) (`self.Lift_Current_Location`) false false))

(event `self.Cube.OnClicked`
  (params (TouchedComponent :type "PrimitiveComponent Object Reference") (ButtonPressed :type "Key Structure"))
  (if (`self.Is_At_A`)
    (`self.Go to B`)
    (else
      (`self.Go to A`))))

(event `self.Box.OnComponentBeginOverlap`
  (params (OverlappedComponent :type "PrimitiveComponent Object Reference") (OtherActor :type "Actor Object Reference") (OtherComp :type "PrimitiveComponent Object Reference") (OtherBodyIndex :type Integer) (bFromSweep :type Boolean) (SweepResult :type "HitResult Structure (by ref)"))
  (cast `Pawn` OtherActor)
  (set `self.IsInRange` true)
  (`KismetSystemLibrary.PrintString` "In Range"))

(event `self.Box.OnComponentEndOverlap`
  (params (OverlappedComponent :type "PrimitiveComponent Object Reference") (OtherActor :type "Actor Object Reference") (OtherComp :type "PrimitiveComponent Object Reference") (OtherBodyIndex :type Integer))
  (set `self.IsInRange` false)
  (`KismetSystemLibrary.PrintString` "In Out of Range"))

(event `Go to A`
  ;[1 1 1] Initate Actions
  (if (`self.IsInRange`)
    (set `self.Is_At_A` true)
    (if (not (`self.Is_Locked`)) :!label _label
      (`GameplayStatics.PlaySound2D` "/Game/Ricardo/Audio/SFX/ES_Sci_Fi_Spaceship_10_-_SFX_Producer.ES_Sci_Fi_Spaceship_10_-_SFX_Producer" 0.7 1.0 0.0 null null)
      (if (`TimelineComponent.IsPlaying` (`self.Lift_Timeline`))
        (bind (_direction _newtrack_0) (`Timeline|Lift_Timeline` :!label _label_2)
          (:`Update`
            (`SceneComponent.K2_SetRelativeLocation` (`self.Lift_Platform_Main`) (`KismetMathLibrary.VLerp` (`self.Point_B_Location`) (`self.Point_A_Location`) _newtrack_0) false false)))
        (else
          (goto _label_2 :!via `PlayFromStart`))))))

(event `self.BPC_InteractionActor_Goto_A.StartAction`
  ;[1 1 1] Initate Actions
  (goto _label))

(event `Go to B`
  ;[1 1 1] Initate Actions
  (if (`self.IsInRange`)
    (set `self.Is_At_A` false)
    (if (not (`self.Is_Locked`)) :!label _label_3
      (`GameplayStatics.PlaySound2D` "/Game/Ricardo/Audio/SFX/ES_Sci_Fi_Spaceship_10_-_SFX_Producer.ES_Sci_Fi_Spaceship_10_-_SFX_Producer" 0.7 0.8 0.0 null null)
      (if (`TimelineComponent.IsPlaying` (`self.Lift_Timeline`))
        (goto _label_2 :!via `Reverse`)
        (else
          (goto _label_2 :!via `ReverseFromEnd`))))))

(event `self.BPC_InteractionActor_Goto_B.StartAction`
  ;[1 1 1] Initate Actions
  (goto _label_3))

(fn `UserConstructionScript`)