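; BP_NPC_Character is a friendly NPC with a character type that the player can interact with.
; A tagged-player overlap sphere stores the player reference and toggles a speech widget animation, resetting the interaction trigger on exit.
; Interacting sends the player a friendly-character message with the NPC's type and reference.
; Construction selects mesh and AnimBP by type, currently identical for all assigned types; Tick displays the type name on a TextRender.
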(event `self.ReceiveBeginPlay`
  (bind _ashud_basic_speech (cast `/Game/Dan/TopDownBP/UI/HUD_BasicSpeech` (`WidgetComponent.GetUserWidgetObject` (`self.Widget`))))
  (bind _output_get (set `self.HUD_Text` _ashud_basic_speech))
  (`/Game/Dan/TopDownBP/UI/HUD_BasicSpeech.SetText` _output_get "Friieeeend!"))

(event `self.Sphere.OnComponentBeginOverlap`
  (params (OverlappedComponent :type "PrimitiveComponent Object Reference") (OtherActor :type "Actor Object Reference") (OtherComp :type "PrimitiveComponent Object Reference") (OtherBodyIndex :type Integer) (bFromSweep :type Boolean) (SweepResult :type "HitResult Structure (by ref)"))
  (if (`ActorComponent.ComponentHasTag` OtherComp "Player")
    (set `self.CharacterRef` OtherActor)
    (`/Game/Dan/TopDownBP/UI/HUD_BasicSpeech.StartAnim` (`self.HUD_Text`) true)))

(event `self.Sphere.OnComponentEndOverlap`
  (params (OverlappedComponent :type "PrimitiveComponent Object Reference") (OtherActor :type "Actor Object Reference") (OtherComp :type "PrimitiveComponent Object Reference") (OtherBodyIndex :type Integer))
  (if (`ActorComponent.ComponentHasTag` OtherComp "Player")
    (set `self.CharacterRef` null)
    (`/Game/Dan/TopDownBP/UI/HUD_BasicSpeech.StartAnim` (`self.HUD_Text`) false)
    (`/Game/Dan/TopDownBP/Blueprints/Components/Interactions/BPC_InteractionTrigger.Reset` (`self.BPC_InteractionTrigger`))))

(event `self.BPC_InteractionTrigger.OnInteract`
  (params (On :type Boolean))
  (bind _characterref (`self.CharacterRef`)
    (:`then`
      (message `/Game/Dan/TopDownBP/Blueprints/Interfaces/Inter_Player.Add Friendly Character` _characterref (`self.CharacterType`) self))
    (:`else`)))

(event `self.ReceiveTick`
  (params (DeltaSeconds :type "Float (single-precision)"))
  (`TextRenderComponent.K2_SetText` (`self.TextRender`) (`KismetTextLibrary.Conv_StringToText` (`|GetEnumeratorNameAsString` (`self.CharacterType`)))))

(fn `UserConstructionScript`
  (bind _charactertype (`self.CharacterType`))
  (bind _body (`self.Body`))
  (`SkinnedMeshComponent.SetSkinnedAssetAndUpdate` _body (select `/Game/Dan/TopDownBP/Blueprints/Enums/E_BotType` _charactertype :`NewEnumerator2` "/Game/SCK_Casual01/Models/Premade_Characters/MESH_PC_02.MESH_PC_02" :`NewEnumerator0` "/Game/SCK_Casual01/Models/Premade_Characters/MESH_PC_02.MESH_PC_02" :`NewEnumerator4` "/Game/SCK_Casual01/Models/Premade_Characters/MESH_PC_02.MESH_PC_02" :`NewEnumerator3` "/Game/SCK_Casual01/Models/Premade_Characters/MESH_PC_02.MESH_PC_02" :!type "SkeletalMesh Object Reference") true)
  (`SkeletalMeshComponent.SetAnimInstanceClass` _body (select `/Game/Dan/TopDownBP/Blueprints/Enums/E_BotType` _charactertype :`NewEnumerator2` "/Game/SCK_Casual01/Mannequin/Animations/ThirdPerson_AnimBP1.ThirdPerson_AnimBP1_C" :`NewEnumerator0` "/Game/SCK_Casual01/Mannequin/Animations/ThirdPerson_AnimBP1.ThirdPerson_AnimBP1_C" :`NewEnumerator4` "/Game/SCK_Casual01/Mannequin/Animations/ThirdPerson_AnimBP1.ThirdPerson_AnimBP1_C" :`NewEnumerator3` "/Game/SCK_Casual01/Mannequin/Animations/ThirdPerson_AnimBP1.ThirdPerson_AnimBP1_C" :!type "Object Class Reference"))
  (`SceneComponent.SetRelativeScale3D` _body (1.0 1.0 1.0)))