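; Player character that switches between squad character types on keys 1-4 by swapping places with the active friendly of that type.
; ChangeCharacter teleports the player to that actor, destroys it, spawns BP_NPC_Character as the previous type and updates the ActiveCharacterTypes map.
; Per-type data maps set mesh, anim class, speeds, multipliers and two ability function names.
; Ability inputs call those names through timers; Stun, Carry and Hack only print.
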(event `self.ReceiveBeginPlay`
  (`PlayerController.SetViewTargetWithBlend` (`GameplayStatics.GetPlayerController` 0) self 0.0 "VTBlend_Linear" 0.0 false)
  (set `PlayerController.bShowMouseCursor` true (`GameplayStatics.GetPlayerController` 0))
  (message `/Game/Dan/TopDownBP/Blueprints/Interfaces/Inter_Player.ToggleMove` (`GameplayStatics.GetPlayerController` 0) false)
  (`PrimitiveComponent.SetRenderCustomDepth` (`self.Mesh`) true)
  (`ActorComponent.Activate` (`self.Camera`) false)
  (`BlueprintMapLibrary.Map_Add` (`self.ActiveCharacterTypes`) "NewEnumerator4" self))

(event `/Game/Dan/TopDownBP/Blueprints/Interfaces/Inter_Player.Add Friendly Character`
  (params (InCharacterType :type "/Game/Dan/TopDownBP/Blueprints/Enums/E_BotType Enum" :default "NewEnumerator5") (InCharacter :type "Actor Object Reference"))
  (`BlueprintMapLibrary.Map_Add` (`self.ActiveCharacterTypes`) InCharacterType InCharacter))

(event `Key|One` :consume false
  (params (Key :type "Key Structure"))
  (:`Pressed`
    (`self.EqualToCurrentCharacter` "NewEnumerator4"
      (:`NewCharacterType`
        (`self.ChangeCharacter` "NewEnumerator4")))))

(event `InputAction|1stAbility`
  (params (Key :type "Key Structure"))
  (bind _1stactivefunctionname (`self.1stActiveFunctionName`))
  (:`Pressed`
    (`KismetSystemLibrary.K2_SetTimer` null _1stactivefunctionname 0.001)
    (`KismetSystemLibrary.PrintString` _1stactivefunctionname true true (struct :`G` 0.66 :`B` 1.0 :`A` 1.0) 20.0)))

(event `Key|Two` :consume false
  (params (Key :type "Key Structure"))
  (:`Pressed`
    (`self.EqualToCurrentCharacter` "NewEnumerator3"
      (:`NewCharacterType`
        (`self.ChangeCharacter` "NewEnumerator3")))))

(event `InputAction|2ndAbiliy`
  (params (Key :type "Key Structure"))
  (bind _2ndactivefunctionname (`self.2ndActiveFunctionName`))
  (:`Pressed`
    (`KismetSystemLibrary.K2_SetTimer` null _2ndactivefunctionname 0.001)
    (`KismetSystemLibrary.PrintString` _2ndactivefunctionname true true (struct :`G` 0.66 :`B` 1.0 :`A` 1.0) 20.0)))

(event `Key|Three` :consume false
  (params (Key :type "Key Structure"))
  (:`Pressed`
    (`self.EqualToCurrentCharacter` "NewEnumerator0"
      (:`NewCharacterType`
        (`self.ChangeCharacter` "NewEnumerator0")))))

(event `Key|Four` :consume false
  (params (Key :type "Key Structure"))
  (:`Pressed`
    (`self.EqualToCurrentCharacter` "NewEnumerator2"
      (:`NewCharacterType`
        (`self.ChangeCharacter` "NewEnumerator2")))))

(fn `AskCameraSetting`
  (returns (FOV :type "Float (double-precision)") (SpringArm :type "Float (double-precision)"))
  (return 0.0 0.0))

(fn `AskPowerAmount`
  (returns (Amount :type Integer))
  (return 0))

(fn `CanAssimilate`
  (returns (Yes :type Boolean))
  (return false))

(fn `CanPushPull?`
  (returns (Yes :type Boolean))
  (return false))

(fn `Carry`
  (`KismetSystemLibrary.PrintString` "CARRYING!!!!!!!!!!!!!!" true true (struct :`G` 0.66 :`B` 1.0 :`A` 1.0) 10.0))

(fn `ChangeCharacter`
  (params (InCharacterType :type "/Game/Dan/TopDownBP/Blueprints/Enums/E_BotType Enum" :default "NewEnumerator5"))
  (locals (LocalTargetTransform :type "Transform Structure") (LocalCurrentTransform :type "Transform Structure") (LocalTargetActor :type "Actor Object Reference") (LocalPreviousCharacterType :type "/Game/Dan/TopDownBP/Blueprints/Enums/E_BotType Enum" :default "NewEnumerator5"))
  (bind (_localtargettransform_location _localtargettransform_rotation) (`KismetMathLibrary.BreakTransform` (`local.LocalTargetTransform`)))
  (bind (_value _returnvalue) (`BlueprintMapLibrary.Map_Find` (`self.ActiveCharacterTypes`) InCharacterType))
  (if _returnvalue
    (`|ExecutionSequence`
      (:`then_0`
        (bind _output_get (set `local.LocalTargetActor` _value))
        (set `local.LocalTargetTransform` (`self.GetTransform` _output_get))
        (`BlueprintMapLibrary.Map_Remove` (`self.ActiveCharacterTypes`) (`self.CurrentCharacterType`))
        (`BlueprintMapLibrary.Map_Remove` (`self.ActiveCharacterTypes`) (`local.InCharacterType`))
        (set `local.LocalPreviousCharacterType` (`self.CurrentCharacterType`))
        (set `self.CurrentCharacterType` (`local.InCharacterType`))
        (set `local.LocalCurrentTransform` (`self.GetTransform`))
        (`KismetSystemLibrary.PrintString` "Change Character"))
      (:`then_1`
        (`self.K2_TeleportTo` _localtargettransform_location _localtargettransform_rotation)
        (`BlueprintMapLibrary.Map_Add` (`self.ActiveCharacterTypes`) (`local.InCharacterType`) self)
        (`self.K2_DestroyActor` (`local.LocalTargetActor`))
        (bind _returnvalue_2 (`|SpawnActorFromClass` "/Game/Dan/Temp/BP_NPC_Character.BP_NPC_Character_C" (`local.LocalCurrentTransform`) "Undefined" "OverrideRootScale" null (`local.LocalPreviousCharacterType`) null))
        (`BlueprintMapLibrary.Map_Add` (`self.ActiveCharacterTypes`) (`local.LocalPreviousCharacterType`) _returnvalue_2)
        (`self.SetMeshAnims` (`local.InCharacterType`))
        (`self.SetCharacterAbilities` (`local.InCharacterType`))))
    (else
      (`KismetSystemLibrary.PrintString` "Character Not Active"))))

(fn `Hack`
  (`KismetSystemLibrary.PrintString` "HACKING!!!!!!!!!!!!!!" true true (struct :`G` 0.66 :`B` 1.0 :`A` 1.0) 10.0))

(fn `IsCanJumpActive`
  (returns (`Jump?` :type Boolean))
  (return false))

(fn `SetCharacterAbilities`
  (params (InCharacterType :type "/Game/Dan/TopDownBP/Blueprints/Enums/E_BotType Enum" :default "NewEnumerator5"))
  (locals (LocalAbility :type "/Game/Dan/Temp/ST_CharacterAbilities Structure"))
  (bind _output_get (set `local.LocalAbility` (`BlueprintMapLibrary.Map_Find` (`self.CharacterAbilities`) InCharacterType)))
  (bind (_maxwalkspeed _maxrunspeed _maxcrouchspeed _maxcarryspeed _movementnoisemultiplier _healthmultiplier _1stactivefunctionname _2ndactivefunctionname) (break `/Game/Dan/Temp/ST_CharacterAbilities` _output_get))
  (set `self.MaxWalkSpeed` _maxwalkspeed)
  (set `self.MaxRunSpeed` _maxrunspeed)
  (set `self.MaxCrouchSpeed` _maxcrouchspeed)
  (set `self.MaxCarrySpeed` _maxcarryspeed)
  (set `self.MovementNoiseMultiplier` _movementnoisemultiplier)
  (set `self.HealthMultiplier` _healthmultiplier)
  (set `self.1stActiveFunctionName` _1stactivefunctionname)
  (set `self.2ndActiveFunctionName` _2ndactivefunctionname))

(fn `SetMeshAnims`
  (params (InCharacterType :type "/Game/Dan/TopDownBP/Blueprints/Enums/E_BotType Enum" :default "NewEnumerator5"))
  (locals (LocalCharacterData :type "/Game/Dan/Temp/ST_UpdateCharacterMesh Structure"))
  (bind _output_get (set `local.LocalCharacterData` (`BlueprintMapLibrary.Map_Find` (`self.CharacterMeshData`) InCharacterType)))
  (`SkinnedMeshComponent.SetSkinnedAssetAndUpdate` (`self.Mesh`) (`.CharacterMesh_4_BD54F047464572A89D8ADB8ED7472C73` (break `/Game/Dan/Temp/ST_UpdateCharacterMesh` _output_get)) true)
  (`SkeletalMeshComponent.SetAnimInstanceClass` (`self.Mesh`) (`.CharacterAnimClass_5_E1A265E048B9E9E2CF2BA1AF9D9CBD12` (break `/Game/Dan/Temp/ST_UpdateCharacterMesh` (`local.LocalCharacterData`)))))

(fn `Stun`
  (`KismetSystemLibrary.PrintString` "STUNNNG!!!!!!!!!!!!!!" true true (struct :`G` 0.66 :`B` 1.0 :`A` 1.0) 10.0))

(fn `UserConstructionScript`
  (`self.SetMeshAnims` (`self.CurrentCharacterType`))
  (`self.SetCharacterAbilities` (`self.CurrentCharacterType`)))

(fn `WhichMainPart`
  (returns (MainPart :type "/Game/Dan/TopDownBP/Blueprints/Enums/E_BotType Enum"))
  (return "NewEnumerator5"))